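; BP_Grid is an actor that lays out a flat grid of static mesh tiles around its own position.
; The construction script runs nested loops over Rows and Cols, centered on zero, and adds one thin, flattened mesh component per cell, spaced by SizeBox.
; Tile offsets are computed in world axes from the actor location, then converted to relative positions by subtracting it; the event graph has no active logic.
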(event EventBeginPlay)

(event Collision|EventActorBeginOverlap
  (params (OtherActor :type Actor%20Object%20Reference)))

(event EventTick
  (params (DeltaSeconds :type Float%20%28single-precision%29)))

(fn ConstructionScript
  (bind _returnvalue (Transformation|GetActorLocation))
  (bind _rows (Variables|Default|GetRows))
  (bind _cols (Variables|Default|GetCols))
  (bind _returnvalue_2 (/ _rows 2.0))
  (bind _returnvalue_3 (/ _cols 2.0))
  (LocalVariables|SetBaseX (.x _returnvalue))
  (LocalVariables|SetBaseY (.y _returnvalue))
  (for _index (range (Math|Float|Truncate (* _returnvalue_2 -1.0)) (Math|Float|Truncate (- _returnvalue_2 1.0)))
    (LocalVariables|SetRowNumber _index)
    (for _index_2 (range (Math|Float|Truncate (* _returnvalue_3 -1.0)) (Math|Float|Truncate (- _returnvalue_3 1.0)))
      (LocalVariables|SetColNumber _index_2)
      (AddComponent|AddStaticMeshComponent false (Math|Transform|MakeTransform (- (Math|Vector|MakeVector (+ (LocalVariables|GetBaseX) (* (LocalVariables|GetRowNumber) (Variables|Default|GetSizeBox))) (+ (LocalVariables|GetBaseY) (* (LocalVariables|GetColNumber) (Variables|Default|GetSizeBox))) (.z (Transformation|GetActorLocation))) (Transformation|GetActorLocation)) "0, 0, 0" "10.000000,10.000000,0.100000")))))