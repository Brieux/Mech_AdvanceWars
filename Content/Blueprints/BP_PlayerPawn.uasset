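; Player pawn for a top-down boat game: world-axis camera panning, zoom, and click-to-command unit control.
; Select traces under the cursor for a BP_Bato; action sends it to the hit mesh's location, randomly via GoThereX or GoThereY.
; Zoom clamps camera FOV and lerps pawn height from it, logic BeginPlay reuses after creating the UI_BateauPoint widget.
; Deselection logic is unwired, so previously selected boats are never deselected here.
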(event Custom|SetFirstPlace
  (bind _returnvalue (Transformation|GetActorLocation))
  (bind _camera (Variables|Default|GetCamera))
  (Camera|SetFieldOfView _camera (Math|Float|Clamp(Float) (+ (Variables|/Script/Engine.CameraComponent|GetFieldOfView _camera) (* (stale Input|EnhancedActionEvents|EnhancedInputActionIA_Zoom ActionValue) -1.0)) 8e+01 1.1e+02))
  (Transformation|SetActorLocation self (Math|Vector|MakeVector (.x _returnvalue) (.y _returnvalue) (Math|Float|Lerp (Variables|Default|GetMinDistZ) (Variables|Default|GetMaxDistZ) (Math|Float|NormalizetoRange (Math|Float|Clamp(Float) (+ (Variables|/Script/Engine.CameraComponent|GetFieldOfView _camera) (* (stale Input|EnhancedActionEvents|EnhancedInputActionIA_Zoom ActionValue) -1.0)) 8e+01 1.1e+02) 8e+01 1.1e+02))) false false))

(event Input|EnhancedActionEvents|EnhancedInputActionIA_MoveF
  (params (ActionValue :type Float%20%28double-precision%29) (ElapsedSeconds :type Float%20%28double-precision%29) (TriggeredSeconds :type Float%20%28double-precision%29) (InputAction :type Input%20Action%20Object%20Reference :default "/Game/Blueprints/Input/IA_MoveF.IA_MoveF"))
  (:Triggered
    (Pawn|Input|AddMovementInput "1.000000,0.000000,0.000000" ActionValue false)))

(event Input|EnhancedActionEvents|EnhancedInputActionIA_MoveL
  (params (ActionValue :type Float%20%28double-precision%29) (ElapsedSeconds :type Float%20%28double-precision%29) (TriggeredSeconds :type Float%20%28double-precision%29) (InputAction :type Input%20Action%20Object%20Reference :default "/Game/Blueprints/Input/IA_MoveL.IA_MoveL"))
  (:Triggered
    (Pawn|Input|AddMovementInput "0.000000,1.000000,0.000000" ActionValue false)))

(event Input|EnhancedActionEvents|EnhancedInputActionIA_SelectUnit
  (params (ActionValue :type Boolean) (ElapsedSeconds :type Float%20%28double-precision%29) (TriggeredSeconds :type Float%20%28double-precision%29) (InputAction :type Input%20Action%20Object%20Reference :default "/Game/Blueprints/Input/IA_SelectUnit.IA_SelectUnit"))
  (:Started
    (bind _asbp_bato (Utilities|Casting|CastToBP_Bato (.HitActor (Collision|BreakHitResult (.HitResult (Game|Player|GetHitResultUnderCursorbyChannel (Game|GetPlayerController 0) "TraceTypeQuery1" true))))))
    (Default|IsSelected _asbp_bato true)
    (Variables|Default|SetIsSelect _asbp_bato)))

(event Input|EnhancedActionEvents|EnhancedInputActionIA_Zoom
  (params (ActionValue :type Float%20%28double-precision%29) (ElapsedSeconds :type Float%20%28double-precision%29) (TriggeredSeconds :type Float%20%28double-precision%29) (InputAction :type Input%20Action%20Object%20Reference :default "/Game/Blueprints/Input/IA_Zoom.IA_Zoom"))
  (bind _returnvalue (Transformation|GetActorLocation))
  (bind _returnvalue_2 (* ActionValue -1.0))
  (bind _camera (Variables|Default|GetCamera))
  (bind _fieldofview (Variables|/Script/Engine.CameraComponent|GetFieldOfView _camera))
  (bind _returnvalue_3 (+ _fieldofview _returnvalue_2))
  (bind _returnvalue_4 (Math|Float|Clamp(Float) _returnvalue_3 8e+01 1.1e+02))
  (:Triggered
    (Camera|SetFieldOfView _camera _returnvalue_4)
    (Transformation|SetActorLocation self (Math|Vector|MakeVector (.x _returnvalue) (.y _returnvalue) (Math|Float|Lerp (Variables|Default|GetMinDistZ) (Variables|Default|GetMaxDistZ) (Math|Float|NormalizetoRange _returnvalue_4 8e+01 1.1e+02))) false false)))

(event Input|EnhancedActionEvents|EnhancedInputActionIA_Action
  (params (ActionValue :type Boolean) (ElapsedSeconds :type Float%20%28double-precision%29) (TriggeredSeconds :type Float%20%28double-precision%29) (InputAction :type Input%20Action%20Object%20Reference :default "/Game/Blueprints/Input/IA_Action.IA_Action"))
  (bind _isselect (Variables|Default|GetIsSelect))
  (:Started
    (Utilities|IsValid (Variables|Default|GetIsSelect)
      (:Is%20Valid
        (bind _asstatic_mesh_component (Utilities|Casting|CastToStaticMeshComponent (.hitcomponent (.HitResult (Game|Player|GetHitResultUnderCursorbyChannel (Game|GetPlayerController 0) "TraceTypeQuery3" true)))))
        (if (Math|Random|RandomBool)
          (Default|GoThereX _isselect (Transformation|GetWorldLocation _asstatic_mesh_component) true)
          (else
            (Default|GoThereY _isselect (Transformation|GetWorldLocation _asstatic_mesh_component) true)))))))

(event Collision|EventActorBeginOverlap
  (params (OtherActor :type Actor%20Object%20Reference)))

(event EventTick
  (params (DeltaSeconds :type Float%20%28single-precision%29)))

(event EventBeginPlay
  (bind _returnvalue (UserInterface|CreateWidget "/Game/UI_BateauPoint.UI_BateauPoint_C"))
  (bind _output_get (Variables|Default|SetUI_Ref _returnvalue))
  (UserInterface|Viewport|AddtoPlayerScreen _output_get)
  (CallFunction|SetFirstPlace))

(fn ConstructionScript)