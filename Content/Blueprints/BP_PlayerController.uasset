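; Player controller that detects when the mouse cursor reaches the screen edges, apparently for edge-scroll movement.
; On possess it adds the IMC_Play Enhanced Input mapping context and shows the cursor.
; Each tick it compares mouse position to the viewport bounds inset by OffSet, setting NeedToMove and, only while that is true, four directional flags.
; It applies no movement itself.
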(event EventTick
  (params (DeltaSeconds :type Float%20%28single-precision%29))
  (bind (_sizex _sizey) (HUD|GetViewportSize))
  (bind (_locationx _locationy) (Game|Player|GetMousePosition))
  (bind _offset (Variables|Default|GetOffSet))
  (bind _offset_2 (Variables|Default|GetOffSet))
  (bind _returnvalue (<= _locationy _offset_2))
  (bind _returnvalue_2 (<= _locationx _offset))
  (bind _returnvalue_3 (- _sizey _offset_2))
  (bind _returnvalue_4 (- _sizex _offset))
  (bind _returnvalue_5 (>= _locationy _returnvalue_3))
  (bind _returnvalue_6 (>= _locationx _returnvalue_4))
  (bind _output_get (Variables|Default|SetneedToMove (or (or _returnvalue_2 _returnvalue_6) (or _returnvalue _returnvalue_5))))
  (if _output_get
    (Variables|Default|SetMoveTop _returnvalue)
    (Variables|Default|SetMoveBot _returnvalue_5)
    (Variables|Default|SetMoveRight _returnvalue_6)
    (Variables|Default|SetMoveLeft _returnvalue_2)))

(event EventPossess
  (params (PossessedPawn :type Pawn%20Object%20Reference))
  (Input|AddMappingContext (PlayerController|LocalPlayerSubsystems|GetEnhancedInputLocalPlayerSubsystem) "/Game/Blueprints/Input/IMC_Play.IMC_Play" 0 "(bIgnoreAllPressedKeysUntilRelease=True,bForceImmediately=False)")
  (Variables|Default|SetbShowMouseCursor true))

(fn ConstructionScript)