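; BP_Bato is a selectable boat actor that moves along X and Y one axis at a time, spending action points (PA).
; GoThereX and GoThereY lerp location by timeline while turning toward the target, then chain to the other axis.
; Each leg deducts PA per 1025-unit step, and Tick writes the total to a UI_PA widget.
; Dynamic materials show selection, while focus toggles the Poupe, Pont and Proue components' visibility.
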(event Custom|isSelected
  (params (Select :type Boolean))
  (Rendering|Material|SetScalarParameterValue (Variables|Default|GetMat1) "Slected?" (Math|Float|SelectFloat 1.0 0.0 Select) :!class /Script/Engine.MaterialInstanceDynamic))

(event Custom|GoThereY
  (params (WhereToGo? :type Vector) (First? :type Boolean))
  (bind (_x _y _z) (Class|KismetMathLibrary|BreakVector3f WhereToGo?))
  (bind _output_get (Variables|Default|SetDeb (Transformation|GetActorLocation)))
  (Variables|Default|SetFin (Math|Vector|MakeVector (.x _output_get) _y _z))
  (if (and (== (.y _output_get) _y) First?)
    (CallFunction|GoThereX WhereToGo? false)
    (else
      (CallFunction|PACost)
      (Components|Timeline|SetPlayRate (Variables|Default|GetTimeline_0) (Variables|Default|GetSpeed))
      (bind _newtrack_0 (Timeline|Timeline_0 PlayFromStart)
        (:Update
          (Transformation|SetActorLocation (Math|Vector|Lerp(Vector) (Variables|Default|GetDeb) (Variables|Default|GetFin) _newtrack_0) false false)
          (Transformation|SetActorRotation (Math|Interpolation|RInterpTo (Transformation|GetActorRotation) (Math|Rotator|FindLookatRotation (Variables|Default|GetDeb) (Variables|Default|GetFin)) (Utilities|Time|GetWorldDeltaSeconds) 15.0)))
        (:Finished
          (if First?
            (CallFunction|GoThereX WhereToGo? false)))))))

(event Custom|PACost
  (bind _deb (Variables|Default|GetDeb))
  (bind _fin (Variables|Default|GetFin))
  (Variables|Default|SetPA (- (Variables|Default|GetPA) (+ (Math|Float|Truncate (/ (Math|Float|Absolute(Float) (- (.x _deb) (.x _fin))) 1025.0)) (Math|Float|Truncate (/ (Math|Float|Absolute(Float) (- (.y _deb) (.y _fin))) 1025.0))))))

(event Custom|GoThereX
  (params (WhereToGo? :type Vector) (First? :type Boolean))
  (bind (_x _y _z) (Class|KismetMathLibrary|BreakVector3f WhereToGo?))
  (bind _output_get (Variables|Default|SetDeb (Transformation|GetActorLocation)))
  (Variables|Default|SetFin (Math|Vector|MakeVector _x (.y _output_get) _z))
  (if (and (== (.x _output_get) _x) First?)
    (CallFunction|GoThereY WhereToGo? false)
    (else
      (CallFunction|PACost)
      (Components|Timeline|SetPlayRate (Variables|Default|GetTimeline) (Variables|Default|GetSpeed))
      (bind _newtrack_0 (Timeline|Timeline PlayFromStart)
        (:Update
          (Transformation|SetActorLocation (Math|Vector|Lerp(Vector) (Variables|Default|GetDeb) (Variables|Default|GetFin) _newtrack_0) false false)
          (Transformation|SetActorRotation (Math|Interpolation|RInterpTo (Transformation|GetActorRotation) (Math|Rotator|FindLookatRotation (Variables|Default|GetDeb) (Variables|Default|GetFin)) (Utilities|Time|GetWorldDeltaSeconds) 15.0)))
        (:Finished
          (if First?
            (CallFunction|GoThereY WhereToGo? false)))))))

(event Custom|isInFocus
  (params (Yes :type Boolean))
  (Rendering|SetVisibility (Variables|Default|GetPoupe) Yes false))

(event EventBeginPlay
  (bind _returnvalue (Rendering|Material|CreateDynamicMaterialInstance "/Game/Bateau/Boat_Inst.Boat_Inst" "None" "None" :!class /Script/Engine.KismetMaterialLibrary))
  (Variables|Default|SetMat1 _returnvalue)
  (bind _returnvalue_2 (Rendering|Material|CreateDynamicMaterialInstance "/Game/Bateau/Boat_2_Inst.Boat_2_Inst" "None" "None" :!class /Script/Engine.KismetMaterialLibrary))
  (Variables|Default|SetMat2 _returnvalue_2)
  (Rendering|Material|SetMaterial (Variables|Default|GetStaticMesh) 0 (Variables|Default|GetMat1))
  (Rendering|Material|SetMaterial (Variables|Default|GetStaticMesh) 1 (Variables|Default|GetMat2))
  (bind _returnvalue_3 (Rendering|Material|CreateDynamicMaterialInstance "/Game/Bateau/BoxLine.BoxLine" "None" "None" :!class /Script/Engine.KismetMaterialLibrary))
  (Variables|Default|SetBox1 _returnvalue_3)
  (bind _returnvalue_4 (Rendering|Material|CreateDynamicMaterialInstance "/Game/Bateau/BoxLine.BoxLine" "None" "None" :!class /Script/Engine.KismetMaterialLibrary))
  (Variables|Default|SetBox2 _returnvalue_4)
  (bind _returnvalue_5 (Rendering|Material|CreateDynamicMaterialInstance "/Game/Bateau/BoxLine.BoxLine" "None" "None" :!class /Script/Engine.KismetMaterialLibrary))
  (Variables|Default|SetBox3 _returnvalue_5)
  (Rendering|Material|SetMaterial (Variables|Default|GetPoupe) 0 (Variables|Default|GetBox1))
  (Rendering|Material|SetMaterial (Variables|Default|GetPont) 0 (Variables|Default|GetBox2))
  (Rendering|Material|SetMaterial (Variables|Default|GetProue) 0 (Variables|Default|GetBox3))
  (Rendering|SetVisibility (Variables|Default|GetPoupe) false false))

(event EventTick
  (params (DeltaSeconds :type Float%20%28single-precision%29))
  (bind _asui_pa (Utilities|Casting|CastToUI_PA (UserInterface|GetWidget (Variables|Default|GetWidget))))
  (Rendering|Components|TextRender|SetText (Variables|/Game/UI_PA.UI_PA_C|GetTextBlock_0 _asui_pa) (Utilities|Text|ToText(Integer) (Variables|Default|GetPA))))

(fn ConstructionScript)